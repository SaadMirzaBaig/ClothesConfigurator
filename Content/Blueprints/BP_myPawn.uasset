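; BP_myPawn is a pawn that shows a configuration UI and lets the player rotate the view by dragging with the mouse.
; On BeginPlay it creates the WBP_CofigUI widget and adds it to the viewport.
; Holding the left mouse button sets a flag that lets the Turn and LookUp axes feed scaled controller yaw and inverted pitch input.
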(event `self.ReceiveBeginPlay`
  (bind _returnvalue (`|CreateWidget` "/Game/Blueprints/WBP_CofigUI.WBP_CofigUI_C"))
  (`UserWidget.AddToViewport` _returnvalue 0))

(event `InputAxis|Turn`
  (params (AxisValue :type "Float (single-precision)"))
  (if (`self.startRotating`)
    (`self.AddControllerYawInput` (* AxisValue 0.7))))

(event `InputAxis|LookUp`
  (params (AxisValue :type "Float (single-precision)"))
  (if (`self.startRotating`)
    (`self.AddControllerPitchInput` (* AxisValue -0.7))))

(event `Key|LeftMouseButton`
  (params (Key :type "Key Structure"))
  (:`Pressed`
    (set `self.startRotating` true))
  (:`Released`
    (set `self.startRotating` false)))

(fn `UserConstructionScript`)